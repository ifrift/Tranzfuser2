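; Heal_BP is an animation notify state in the Witch animation set that applies an area heal effect, labeled "Sphere Ult" in its debug print.
; Each tick runs a debug-drawn sphere trace around the mesh, then calls ApplyDamage on the hit actor using HealAmount from the first Support_BP found.
; Hit actors are added to HitActors, which excludes them from later traces until notify end clears it.
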(fn `Received_NotifyEnd`
  (params (MeshComp :type "SkeletalMeshComponent Object Reference") (Animation :type "AnimSequenceBase Object Reference"))
  (returns (ReturnValue :type Boolean))
  (`KismetArrayLibrary.Array_Clear` (`self.HitActors`))
  (return false))

(fn `Received_NotifyTick`
  (params (MeshComp :type "SkeletalMeshComponent Object Reference") (Animation :type "AnimSequenceBase Object Reference") (FrameDeltaTime :type "Float (double-precision)"))
  (returns (ReturnValue :type Boolean))
  (bind _returnvalue (+ (`SceneComponent.K2_GetComponentLocation` MeshComp) (0.0 0.0 100.0)))
  (`KismetSystemLibrary.PrintString` null "Sphere Ult")
  (bind _outhit (`KismetSystemLibrary.SphereTraceSingle` MeshComp _returnvalue _returnvalue 500.0 "TraceTypeQuery1" false (`self.hitActors`) "ForDuration"))
  (bind _outactors (`GameplayStatics.GetAllActorsOfClass` (`ActorComponent.GetOwner` MeshComp) "/Game/Witch/Witch_Animation_Set/Support_BP.Support_BP_C"))
  (`KismetArrayLibrary.Array_Add` (`self.HitActors`) (`.HitActor` (`GameplayStatics.BreakHitResult` _outhit)))
  (`GameplayStatics.ApplyDamage` (`.HitActor` (`GameplayStatics.BreakHitResult` _outhit)) (`/Game/Witch/Witch_Animation_Set/Support_BP.Heal Amount` (`|GetArrayItem` _outactors)))
  (return false))