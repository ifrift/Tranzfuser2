(event `self.ReceiveBeginPlay`
  (`PrimitiveComponent.IgnoreActorWhenMoving` (`self.Sphere`) (stale `self.ReceiveActorBeginOverlap` _assupport_bp) true))

(event `self.ReceiveActorBeginOverlap`
  (params (OtherActor :type "Actor Object Reference"))
  (`|ExecutionSequence`
    (:`then_0`
      (bind _assupport_bp (cast `/Game/Witch/Witch_Animation_Set/Support_BP` (`self.GetInstigator`)))
      (if (not (`self.ActorHasTag` (`/Game/Witch/Witch_Animation_Set/Support_BP.TeamTag` _assupport_bp)))
        (`|ExecutionSequence`
          (:`then_0`
            (bind _asthird_person_monk (cast `/Game/FighterAnimationPack/ThirdPersonMonk` OtherActor))
            (`GameplayStatics.ApplyDamage` _asthird_person_monk 10.0))
          (:`then_1`
            (bind _asthird_person_character_sam (cast `/Game/Samurai/ThirdPersonCharacterSam` OtherActor))
            (`GameplayStatics.ApplyDamage` _asthird_person_character_sam 10.0))
          (:`then_2`
            (bind _assupport_bp_2 (cast `/Game/Witch/Witch_Animation_Set/Support_BP` OtherActor))
            (`GameplayStatics.ApplyDamage` _assupport_bp_2 10.0)))
        (`self.K2_DestroyActor`)))
    (:`then_1`
      (`GameplayStatics.SpawnEmitterAtLocation` "/Game/More_Effects/AdvancedMagicFX12/particles/P_ky_hit_thunder.P_ky_hit_thunder"))))

(fn `UserConstructionScript`)