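; Fire auto-attack actor from the Witch support attack set that damages enemy heroes it overlaps.
; Its sphere ignores the instigator when moving, and overlaps with any other actor spawn a fire hit effect.
; Targets carrying the instigator's first tag are spared as allies.
; Others tagged Monk, Sam or Support take fixed damage, after which the attack destroys itself.
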(event `self.ReceiveBeginPlay`
  (`PrimitiveComponent.IgnoreActorWhenMoving` (`self.Sphere`) (`self.GetInstigator`) true))

(event `self.ReceiveActorBeginOverlap`
  (params (OtherActor :type "Actor Object Reference"))
  (set `self.HitActor` OtherActor)
  (if (not (== (`self.Instigator`) (`self.HitActor`)))
    (`GameplayStatics.SpawnEmitterAtLocation` "/Game/More_Effects/AdvancedMagicFX12/particles/P_ky_hit_fire.P_ky_hit_fire")
    (if (not (`self.ActorHasTag` (`self.HitActor`) (`|GetArrayItem` (`Actor.Tags` (`self.GetInstigator`)))))
      (`|ExecutionSequence`
        (:`then_0`
          (if (`self.ActorHasTag` (`self.HitActor`) "Monk")
            (`GameplayStatics.ApplyDamage` (`self.HitActor`) 10.0)
            (`self.K2_DestroyActor` :!label _label)))
        (:`then_1`
          (if (`self.ActorHasTag` (`self.HitActor`) "Sam")
            (`GameplayStatics.ApplyDamage` (`self.HitActor`) 10.0)
            (goto _label)))
        (:`then_2`
          (if (`self.ActorHasTag` (`self.HitActor`) "Support")
            (`GameplayStatics.ApplyDamage` (`self.HitActor`) 10.0)
            (goto _label)))))))

(fn `UserConstructionScript`)