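; Earth support attack from the Witch's set that heals allies touching its sphere.
; On overlap, it treats actors carrying the instigator's first tag as allies, then uses Monk, Sam or Support tags to cast and call each class's Heal.
; Every overlap, allied or not, also activates the particle system, which a one-second delay then deactivates.
; The DestroyActor call is unwired, so the actor never destroys itself here.
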(event `self.Sphere.OnComponentBeginOverlap`
  (params (OverlappedComponent :type "PrimitiveComponent Object Reference") (OtherActor :type "Actor Object Reference") (OtherComp :type "PrimitiveComponent Object Reference") (OtherBodyIndex :type Integer) (bFromSweep :type Boolean) (SweepResult :type "HitResult Structure (by ref)"))
  (set `self.HitActor` OtherActor)
  (`|ExecutionSequence`
    (:`then_0`
      (if (`self.ActorHasTag` (`self.HitActor`) (`|GetArrayItem` (`Actor.Tags` (`self.GetInstigator`))))
        (`|ExecutionSequence`
          (:`then_0`
            (if (`self.ActorHasTag` (`self.HitActor`) "Monk")
              (bind _asthird_person_monk (cast `/Game/FighterAnimationPack/ThirdPersonMonk` (`self.HitActor`)))
              (`/Game/FighterAnimationPack/ThirdPersonMonk.Heal` _asthird_person_monk)))
          (:`then_1`
            (if (`self.ActorHasTag` (`self.HitActor`) "Sam")
              (bind _asthird_person_character_sam (cast `/Game/Samurai/ThirdPersonCharacterSam` (`self.HitActor`)))
              (`/Game/Samurai/ThirdPersonCharacterSam.Heal` _asthird_person_character_sam)))
          (:`then_2`
            (if (`self.ActorHasTag` (`self.HitActor`) "Support")
              (bind _assupport_bp (cast `/Game/Witch/Witch_Animation_Set/Support_BP` (`self.HitActor`)))
              (`/Game/Witch/Witch_Animation_Set/Support_BP.Heal` _assupport_bp))))))
    (:`then_1`
      (`ActorComponent.Activate` (`self.ParticleSystem`) false)
      (`KismetSystemLibrary.Delay` 1.0)
      (`ActorComponent.Deactivate` (`self.ParticleSystem`)))))

(fn `UserConstructionScript`)