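; Water auto-attack actor for the Witch support character, filed under old attacks, that deals damage on contact.
; A sphere overlap ignores the instigator and any actor carrying the instigator's first tag.
; Other actors tagged Monk, Sam or Support take fixed damage and the attack destroys itself, while untagged overlaps leave it alive.
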(event `self.Sphere1.OnComponentBeginOverlap`
  (params (OverlappedComponent :type "PrimitiveComponent Object Reference") (OtherActor :type "Actor Object Reference") (OtherComp :type "PrimitiveComponent Object Reference") (OtherBodyIndex :type Integer) (bFromSweep :type Boolean) (SweepResult :type "HitResult Structure (by ref)"))
  (set `self.HitActor` OtherActor)
  (if (== (`self.Instigator`) (`self.HitActor`))
    _
    (elif (not (`self.ActorHasTag` (`self.HitActor`) (`|GetArrayItem` (`Actor.Tags` (`self.GetInstigator`)))))
      (`|ExecutionSequence`
        (:`then_0`
          (if (`self.ActorHasTag` (`self.HitActor`) "Monk")
            (`GameplayStatics.ApplyDamage` (`self.HitActor`) 10.0)
            (`self.K2_DestroyActor` :!label _label)))
        (:`then_1`
          (if (`self.ActorHasTag` (`self.HitActor`) "Sam")
            (`GameplayStatics.ApplyDamage` (`self.HitActor`) 10.0)
            (goto _label)))
        (:`then_2`
          (if (`self.ActorHasTag` (`self.HitActor`) "Support")
            (`GameplayStatics.ApplyDamage` (`self.HitActor`) 10.0)
            (goto _label)))))))

(fn `UserConstructionScript`)