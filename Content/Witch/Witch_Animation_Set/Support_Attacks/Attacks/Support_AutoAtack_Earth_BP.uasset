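; Damage actor for the Witch Support character's earth auto-attack.
; On capsule overlap it ignores the instigator and any actor sharing the instigator's first tag, apparently as a team filter.
; Targets tagged Monk, Sam or Support each pass through their own DoOnce to take fixed damage.
; A short delay after a hit, the actor destroys itself and resets the DoOnce gates.
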(event `self.Capsule.OnComponentBeginOverlap`
  (params (OverlappedComponent :type "PrimitiveComponent Object Reference") (OtherActor :type "Actor Object Reference") (OtherComp :type "PrimitiveComponent Object Reference") (OtherBodyIndex :type Integer) (bFromSweep :type Boolean) (SweepResult :type "HitResult Structure (by ref)"))
  (set `self.HitActor` OtherActor)
  (if (== (`self.Instigator`) (`self.HitActor`))
    _
    (elif (not (`self.ActorHasTag` (`self.HitActor`) (`|GetArrayItem` (`Actor.Tags` (`self.GetInstigator`)))))
      (`|ExecutionSequence`
        (:`then_0`
          (if (`self.ActorHasTag` (`self.HitActor`) "Monk")
            (`/Engine/EditorBlueprintResources/StandardMacros.DoOnce` false :!label _label
              (:`Completed`
                (`GameplayStatics.ApplyDamage` (`self.HitActor`) 10.0)
                (`KismetSystemLibrary.Delay` 0.2 :!label _label_2)
                (`self.K2_DestroyActor`)
                (`|ExecutionSequence`
                  (:`then_0`
                    (goto _label :!via `Reset`))
                  (:`then_1`
                    (goto _label_3 :!via `Reset`))
                  (:`then_2`
                    (goto _label_4 :!via `Reset`)))))))
        (:`then_1`
          (if (`self.ActorHasTag` (`self.HitActor`) "Sam")
            (`/Engine/EditorBlueprintResources/StandardMacros.DoOnce` false :!label _label_3
              (:`Completed`
                (`GameplayStatics.ApplyDamage` (`self.HitActor`) 10.0)
                (goto _label_2)))))
        (:`then_2`
          (if (`self.ActorHasTag` (`self.HitActor`) "Support")
            (`/Engine/EditorBlueprintResources/StandardMacros.DoOnce` false :!label _label_4
              (:`Completed`
                (`GameplayStatics.ApplyDamage` (`self.HitActor`) 10.0)
                (goto _label_2)))))))))

(fn `UserConstructionScript`)