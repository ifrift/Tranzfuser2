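; Test game state that keeps scores for two teams based on control of Excavator actors.
; On the server, Tick calls a scoring event whose Delay throttles it to roughly five-second intervals.
; Each pass adds a point to a team's score for every Excavator it controls.
; An identical client scoring event exists but has no live caller, and BeginPlay only sets placeholder letter variables.
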(event `self.ReceiveBeginPlay`
  (set `self.A` "A")
  (set `self.B` "B")
  (set `self.C` "C"))

(event `ClientScoreCalulate`
  (`KismetSystemLibrary.Delay` 5.0)
  (bind _outactors (`GameplayStatics.GetAllActorsOfClass` "/Game/ThirdPersonBP/Maps/WhiteBoxBP/Excavator.Excavator_C"))
  (for _array_element _outactors
    (bind _teamcontrolled (`/Game/ThirdPersonBP/Maps/WhiteBoxBP/Excavator.teamControlled` _array_element))
    (if (== _teamcontrolled 1)
      (set `self.teamOneScore` (+ (`self.teamOneScore`) 1))
      (elif (== _teamcontrolled 2)
        (set `self.teamTwoScore` (+ (`self.teamTwoScore`) 1))))))

(event `ServerScoreCalulate`
  (`KismetSystemLibrary.Delay` 5.0)
  (bind _outactors (`GameplayStatics.GetAllActorsOfClass` "/Game/ThirdPersonBP/Maps/WhiteBoxBP/Excavator.Excavator_C"))
  (for _array_element _outactors
    (bind _teamcontrolled (`/Game/ThirdPersonBP/Maps/WhiteBoxBP/Excavator.teamControlled` _array_element))
    (if (== _teamcontrolled 1)
      (set `self.teamOneScore` (+ (`self.teamOneScore`) 1))
      (elif (== _teamcontrolled 2)
        (set `self.teamTwoScore` (+ (`self.teamTwoScore`) 1))))))

(event `self.ReceiveTick`
  (params (DeltaSeconds :type "Float (single-precision)"))
  (if (`KismetSystemLibrary.IsServer`)
    (`self.ServerScoreCalulate`)))

(fn `UserConstructionScript`)