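; Animation notify state for a punch effect that spawns the Nature Slash Niagara system when the notify window begins.
; It places the effect at the mesh's hand_l socket plus FXOffset, despite the RightPunch name.
; Rotation combines the rotation of an unnamed socket with FXRotation, then applies fixed roll and yaw corrections.
; The system spawns at a world location without attaching to the hand.
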(fn `Received_NotifyBegin`
  (params (MeshComp :type "SkeletalMeshComponent Object Reference") (Animation :type "AnimSequenceBase Object Reference") (TotalDuration :type "Float (double-precision)"))
  (returns (ReturnValue :type Boolean))
  (bind (_returnvalue_roll _returnvalue_pitch _returnvalue_yaw) (`KismetMathLibrary.BreakRotator` (`KismetMathLibrary.ComposeRotators` (`SceneComponent.GetSocketRotation` MeshComp "None") (`self.FX_Rotation`))))
  (`NiagaraFunctionLibrary.SpawnSystemAtLocation` MeshComp "/Game/ParticleEffects/Hack_And_Slash_FX/VFX_Niagara/Slashes/NS_Nature_Slash.NS_Nature_Slash" (+ (`SceneComponent.GetSocketLocation` MeshComp "hand_l") (`self.FX_Offset`)) (`KismetMathLibrary.MakeRotator` (+ _returnvalue_roll 180.0) _returnvalue_pitch (+ _returnvalue_yaw -160.0)))
  (return false))