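; Monk earth ultimate effect actor that raises sixteen rocks out of the ground, then removes itself after about six seconds.
; On BeginPlay, downward traces from sixteen cube markers, ignoring the three player character classes, find each rock's surface point and bury it below.
; After a short delay a timeline lerps the rocks up, then reveals a particle system.
; The sphere-trace damage and launch logic is disconnected.
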(event `IgnorePlayerForSpawn`
  ;[1 1 1] Ignore Player When seting start lcoation of Rocks
  (`|ExecutionSequence`
    (:`then_0`
      (bind _outactors (`GameplayStatics.GetAllActorsOfClass` "/Game/FighterAnimationPack/ThirdPersonMonk.ThirdPersonMonk_C"))
      (for _array_element _outactors
        (`KismetArrayLibrary.Array_Add` (`self.IgnoreForSpawn`) _array_element)))
    (:`then_1`
      (bind _outactors_2 (`GameplayStatics.GetAllActorsOfClass` "/Game/Samurai/ThirdPersonCharacterSam.ThirdPersonCharacterSam_C"))
      (for _array_element_2 _outactors_2
        (`KismetArrayLibrary.Array_Add` (`self.IgnoreForSpawn`) _array_element_2)))
    (:`then_2`
      (bind _outactors_3 (`GameplayStatics.GetAllActorsOfClass` "/Game/Witch/Witch_Animation_Set/Support_BP.Support_BP_C"))
      (for _array_element_3 _outactors_3
        (`KismetArrayLibrary.Array_Add` (`self.IgnoreForSpawn`) _array_element_3)))))

(event `SetStart&EndPos`
  (set `self.Rocks` (`|MakeArray` (`self.Rock1`) (`self.Rock2`) (`self.Rock3`) (`self.Rock4`) (`self.Rock5`) (`self.Rock6`) (`self.Rock7`) (`self.Rock8`) (`self.Rock9`) (`self.Rock10`) (`self.Rock11`) (`self.Rock12`) (`self.Rock13`) (`self.Rock14`) (`self.Rock15`) (`self.Rock16`)))
  (for (_array_element _array_index) (`self.ShootDownObject`)
    (bind _returnvalue (`SceneComponent.K2_GetComponentLocation` _array_element))
    (bind _outhit (`KismetSystemLibrary.LineTraceSingle` _returnvalue (- _returnvalue (0.0 0.0 1000.0)) "TraceTypeQuery1" false (`self.IgnoreForSpawn`)))
    (`KismetArrayLibrary.Array_Set` (`self.EndPos`) _array_index (`.ImpactPoint` (`GameplayStatics.BreakHitResult` _outhit)))
    (bind _returnvalue_2 (- (`.ImpactPoint` (`GameplayStatics.BreakHitResult` _outhit)) (0.0 0.0 250.0)))
    (`KismetArrayLibrary.Array_Set` (`self.StartPos`) _array_index _returnvalue_2)
    (`SceneComponent.K2_SetWorldLocation` (`|GetArrayItem` (`self.Rocks`) _array_index) _returnvalue_2 false false)))

(event `self.ReceiveBeginPlay`
  (set `self.ShootDownObject` (`|MakeArray` (`self.Cube1`) (`self.Cube2`) (`self.Cube3`) (`self.Cube4`) (`self.Cube5`) (`self.Cube6`) (`self.Cube7`) (`self.Cube8`) (`self.Cube9`) (`self.Cube10`) (`self.Cube11`) (`self.Cube12`) (`self.Cube13`) (`self.Cube14`) (`self.Cube15`) (`self.Cube16`)))
  (`self.IgnorePlayerForSpawn`)
  (`self.SetStart&EndPos`)
  (`KismetSystemLibrary.Delay` 0.6)
  (bind (_direction _newtrack_0) (`Timeline|RocksUp`)
    (:`Update`
      (`self.RockMovement` (`self.Rocks`) 0 15 _newtrack_0 (`self.StartPos`) (`self.EndPos`))
      (`KismetSystemLibrary.Delay` 6.0)
      (`self.K2_DestroyActor`))
    (:`Finished`
      (`KismetSystemLibrary.Delay` 0.8)
      (`SceneComponent.SetVisibility` (`self.ParticleSystem`) true false))))

(event `RockMovement`
  (params (Rock :type "Array of MeshComponent Object Reference") (FirstIndex :type Integer) (LastIndex :type Integer) (TimelineTime :type "Float (double-precision)") (StartPos :type "Array of Vector Structure") (EndPos :type "Array of Vector Structure"))
  (for (_array_element _array_index) Rock
    (`SceneComponent.K2_SetWorldLocation` _array_element (`KismetMathLibrary.VLerp` (`|GetArrayItem` StartPos _array_index) (`|GetArrayItem` EndPos _array_index) TimelineTime) false false)))

(event `MoveOrder`)

(fn `UserConstructionScript`)