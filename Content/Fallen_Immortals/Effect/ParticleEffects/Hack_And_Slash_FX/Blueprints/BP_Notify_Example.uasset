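; Animation notify state that spawns a Niagara punch effect on the ThirdPersonMonk character when the notify window begins.
; It casts the mesh owner to ThirdPersonMonk and reads its PunchPartEffect system, so other owners get no effect.
; The effect spawns unattached at the spine_02 socket plus FXOffset, with FXRotation combined onto the mesh rotation taken from an unnamed socket lookup.
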(fn `Received_NotifyBegin`
  (params (MeshComp :type "SkeletalMeshComponent Object Reference") (Animation :type "AnimSequenceBase Object Reference") (TotalDuration :type "Float (double-precision)"))
  (returns (ReturnValue :type Boolean))
  (bind _asthird_person_monk (cast `/Game/FighterAnimationPack/ThirdPersonMonk` (`ActorComponent.GetOwner` MeshComp)))
  (`NiagaraFunctionLibrary.SpawnSystemAtLocation` MeshComp (`/Game/FighterAnimationPack/ThirdPersonMonk.PunchPartEffect` _asthird_person_monk) (+ (`SceneComponent.GetSocketLocation` MeshComp "spine_02") (`self.FX_Offset`)) (`KismetMathLibrary.ComposeRotators` (`SceneComponent.GetSocketRotation` MeshComp "None") (`self.FX_Rotation`)))
  (return false))