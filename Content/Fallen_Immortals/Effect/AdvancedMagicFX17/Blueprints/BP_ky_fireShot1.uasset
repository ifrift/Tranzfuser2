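; BP_ky_fireShot1 is an effect actor from the AdvancedMagicFX17 pack that plays the P_ky_fireShot1 fire shot particle at its own location and rotation.
; On BeginPlay it spawns the emitter and passes LengthCorrect into the "vel" vector parameter to adjust shot length.
; After a two-second delay it either respawns the effect when IsLoop is set or destroys itself.
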(event `self.ReceiveBeginPlay`
  ;[1 1 1] effect spawn
  (bind _returnvalue (`GameplayStatics.SpawnEmitterAtLocation` "/Game/Fallen_Immortals/Effect/AdvancedMagicFX17/Particles/P_ky_fireShot1.P_ky_fireShot1" (`self.K2_GetActorLocation` self) (`self.K2_GetActorRotation` self) :!label _label))
  ;[1 1 1] shot length correct
  (`ParticleSystemComponent.SetVectorParameter` _returnvalue "vel" (`KismetMathLibrary.MakeVector` (`KismetMathLibrary.Conv_IntToDouble` (`self.lengthCorrect`))))
  ;[1 1 1] interval
  (`KismetSystemLibrary.Delay` 2.0)
  ;[1 1 1] loop control if true - repeat , if false - destroy
  (if (`self.isLoop`)
    (goto _label)
    (else
      ;[1 1 1] this destroy
      (`self.K2_DestroyActor` self))))

(fn `UserConstructionScript`)