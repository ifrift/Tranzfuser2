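; Rising fire effect actor from the AdvancedMagicFX17 pack, tied to a ThirdPersonMonk instigator.
; BeginPlay captures the Test component's location and the monk's root location, then WaterMove runs a timeline that lerps Fx from the first to the second.
; Tick separately lifts Test by a fixed, frame-rate-dependent step.
; Both endpoints are captured once, so Fx follows neither the monk nor Test afterwards.
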(event `self.ReceiveBeginPlay`
  (set `self.StartPos` (`SceneComponent.K2_GetComponentLocation` (`self.test`)))
  (bind _asthird_person_monk (cast `/Game/FighterAnimationPack/ThirdPersonMonk` (`self.GetInstigator`)))
  (set `self.EndPos` (`SceneComponent.K2_GetComponentLocation` (`Actor.RootComponent` _asthird_person_monk)))
  (`self.WaterMove`))

(event `self.ReceiveTick`
  (params (DeltaSeconds :type "Float (single-precision)"))
  (bind (_returnvalue_x _returnvalue_y _returnvalue_z) (`KismetMathLibrary.BreakVector` (`SceneComponent.K2_GetComponentLocation` (`self.test`))))
  (`SceneComponent.K2_SetWorldLocation` (`self.test`) (`KismetMathLibrary.MakeVector` _returnvalue_x _returnvalue_y (+ _returnvalue_z 100.0)) false false))

(event `WaterMove`
  (bind (_direction _newtrack_0) (`Timeline|Timeline_1` :!via `PlayFromStart`)
    (:`Update`
      (`SceneComponent.K2_SetWorldLocation` (`self.fx`) (`KismetMathLibrary.VLerp` (`self.StartPos`) (`self.EndPos`) _newtrack_0) false false)
      (`KismetSystemLibrary.Delay` 0.8))))

(fn `UserConstructionScript`
  (`parent.UserConstructionScript`))